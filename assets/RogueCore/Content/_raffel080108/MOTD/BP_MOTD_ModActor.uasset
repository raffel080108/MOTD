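; Mod actor for the MOTD mod by raffel080108, which registers the mod's info and UI page.
; On BeginPlay it creates the WBP_MOTD_ModPage widget for the first player controller and binds to the FSD game state's player-leave and character-registered events.
; GetModInfo returns the name, author and version, and GetModUI returns the created page, apparently for a mod hub.
; Both player event handler functions are empty.
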(event EventBeginPlay
  (bind _returnvalue (Class|GameFunctionLibrary|GetFSDGameState))
  (bind _returnvalue_2 (UserInterface|CreateWidget "/Game/_raffel080108/MOTD/UI/Widgets/WBP_MOTD_ModPage.WBP_MOTD_ModPage_C" (Game|GetPlayerController 0)))
  (Variables|Default|SetModHubPage _returnvalue_2)
  (EventDispatchers|BindEventtoOnPlayerLeave _returnvalue (EventDispatchers|CreateEvent :!event FSDGameStateonPlayerLeave))
  (EventDispatchers|BindEventtoOnPlayerCharacterRegistered _returnvalue (EventDispatchers|CreateEvent :!event FSDGameStateonPlayerCharacterRegistered)))

(fn ConstructionScript)

(fn FSDGameStateonPlayerLeave
  (params (PlayerState :type FSD%20Player%20State%20Object%20Reference)))

(fn FSDGameStateonPlayerCharacterRegistered
  (params (PlayerCharacter :type Player%20Character%20Object%20Reference)))

(fn GetModInfo
  (return "MOTD" "raffel080108" "1.0"))

(fn GetModUI
  (return (Utilities|Array|MakeArray (Variables|Default|GetModHubPage))))