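; Entry Blueprint for raffel080108's MOTD mod, exposing its info and settings page to a mod manager.
; On initialise it stores the manager and local player controller, then creates the WBP_MOTD_ModPage widget that GetModUI returns.
; It also binds to FSD game state player-leave and character-registered events, but both handler functions are empty.
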(event EventOnInitialise
  (params (modManager :type BPI%20RC%20Mod%20Manager%20Interface) (localPlayerController :type Player%20Controller%20Object%20Reference))
  (bind _returnvalue (Class|GameFunctionLibrary|GetFSDGameState))
  (Variables|Default|SetModManager modManager)
  (bind _output_get (Variables|Default|SetLocalPlayerController localPlayerController))
  (bind _returnvalue_2 (UserInterface|CreateWidget "/Game/_RCMods/_raffel080108/MOTD/UI/Widgets/WBP_MOTD_ModPage.WBP_MOTD_ModPage_C" _output_get))
  (Variables|Default|SetModPage _returnvalue_2)
  (EventDispatchers|BindEventtoOnPlayerLeave _returnvalue (EventDispatchers|CreateEvent :!event FSDGameStateonPlayerLeave))
  (EventDispatchers|BindEventtoOnPlayerCharacterRegistered _returnvalue (EventDispatchers|CreateEvent :!event FSDGameStateonPlayerCharacterRegistered)))

(fn ConstructionScript)

(fn FSDGameStateonPlayerLeave
  (params (PlayerState :type FSD%20Player%20State%20Object%20Reference)))

(fn FSDGameStateonPlayerCharacterRegistered
  (params (PlayerCharacter :type Player%20Character%20Object%20Reference)))

(fn GetModInfo
  (return "MOTD" "raffel080108" "1.0"))

(fn GetModUI
  (return (Utilities|Array|MakeArray (Variables|Default|GetModPage))))